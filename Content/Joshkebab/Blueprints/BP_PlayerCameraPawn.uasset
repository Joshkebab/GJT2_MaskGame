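; Player camera pawn that follows the level's BP_MaskPLayerPawn, relays click-to-move input and triggers the win screen.
; BeginPlay finds that pawn, adds the input mapping and creates the Glossary widget.
; Tick copies the pawn's location rather than attaching, avoiding inherited rotation, while touches or clicks trace screen-to-world to set its move target.
; At 16 glossary words, once the glossary is closed, it stops ticking and shows W_Win.
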(event Custom|EndGame
  (if (not (Variables|/Game/Ka-ShingFolder/WBP_Glossary.WBP_Glossary_C|GetIsOPen (Variables|Default|GetGlossary)))
    (Actor|Tick|SetActorTickEnabled false)
    (bind _returnvalue (UserInterface|CreateWidget "/Game/Joshkebab/Blueprints/Widgets/W_Win.W_Win_C"))
    (UserInterface|Viewport|AddtoViewport _returnvalue 0)))

(event Input|EnhancedActionEvents|EnhancedInputActionIA_Touch
  (params (ActionValue :type Boolean) (ElapsedSeconds :type Float%20%28double-precision%29) (TriggeredSeconds :type Float%20%28double-precision%29) (InputAction :type Input%20Action%20Object%20Reference :default "/Game/Joshkebab/Input/IA_Touch.IA_Touch"))
  (bind _returnvalue (Game|GetPlayerController 0))
  (bind (_worldlocation _worlddirection) (Game|Player|ConvertMouseLocationToWorldSpace _returnvalue))
  ;[0.4692 1 0.3229] When screen touched or clicked, trace from screen to world and set a new location for the PC to move to.
  (bind _outhit (Collision|LineTraceByChannel _worldlocation (+ _worldlocation (* _worlddirection 1e+05)) "TraceTypeQuery1" false 0 "None"))
  (Default|MovetoTarget (Variables|Default|GetAttachedPlayerPawn) (.Location (Collision|BreakHitResult _outhit))))

(event EventBeginPlay
  ;[1 0.1102 0.09375] I hate doing Get Actor of Class but here this is the easiest way and it's only called once, sue me. Anyway, find the actual player character and add input mappings. ~Kebab
  (bind _returnvalue (Actor|GetActorOfClass "/Game/Joshkebab/Blueprints/BP_MaskPLayerPawn.BP_MaskPLayerPawn_C"))
  (Utilities|IsValid _returnvalue
    (:Is%20Valid
      (Variables|Default|SetAttachedPlayerPawn _returnvalue)
      (Input|AddMappingContext (PlayerController|LocalPlayerSubsystems|GetEnhancedInputLocalPlayerSubsystem (Game|GetPlayerController 0)) "/Game/Joshkebab/Input/IMC_PlayerControls.IMC_PlayerControls" 0 "(bIgnoreAllPressedKeysUntilRelease=True,bForceImmediately=False,bNotifyUserSettings=False)")
      (Variables|Default|SetShouldFollowPlayer true)
      (bind _returnvalue_2 (UserInterface|CreateWidget "/Game/Ka-ShingFolder/WBP_Glossary.WBP_Glossary_C"))
      (bind _output_get (Variables|Default|SetGlossary _returnvalue_2))
      (UserInterface|Viewport|AddtoViewport _output_get 0))
    (:Is%20Not%20Valid
      (Development|PrintString "No BP_MaskPLayerPawn found! Make sure there is exactly one placed in the level where you want the player to start." true true "(R=1.000000,G=0.000000,B=0.040396,A=1.000000)" 1e+02))))

(event EventTick
  (params (DeltaSeconds :type Float%20%28single-precision%29))
  ;[1 0.3777 0.1146] Would do attach, but then it would inheit rotation, nono. This is simpler than finding a different way.
  (if (Variables|Default|GetShouldFollowPlayer)
    (Transformation|SetActorLocation (Transformation|GetActorLocation (Variables|Default|GetAttachedPlayerPawn)) false false)
    (if (== (Variables|/Game/Ka-ShingFolder/WBP_Glossary.WBP_Glossary_C|GetWordProgress (Variables|Default|GetGlossary)) 16)
      (CallFunction|EndGame))))

(event Input|MouseEvents|LeftMouseButton
  (params (Key :type Key%20Structure :default "None")))

(fn ConstructionScript)