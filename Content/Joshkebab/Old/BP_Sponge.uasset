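; BP_Sponge is a sponge actor that follows the mouse cursor to scrub dirt off dishes.
; AttachToMouse and DetachFromMouse toggle tick, a gate and a looping timer.
; While attached, each tick snaps it to the cursor's visibility-trace hit, taking roll and yaw from the surface normal.
; The timer stores cursor travel since the sponge's last sampled location as ScrubValue, then calls CleanTick on the referenced dish.
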(event Custom|AttachToMouse
  (bind _returnvalue (Game|GetPlayerController 0))
  (bind _hitresult (Game|Player|GetHitResultUnderCursorbyChannel _returnvalue "TraceTypeQuery1" true))
  (bind (_bblockinghit _binitialoverlap _time _distance _location _impactpoint _normal _impactnormal) (Collision|BreakHitResult _hitresult))
  (bind _returnvalue_2 (Math|Rotator|MakeRotfromZ _impactnormal))
  ;[1 1 1] Attach the sponge to the mouse and start a timer to progress scrubbing on a dish
  (Actor|Tick|SetActorTickEnabled true)
  (Utilities|Time|SetTimerbyFunctionName 0 "SetScrubValue" 0.1 true)
  (Utilities|FlowControl|Gate true) ; enters at Open
)

(event Custom|DetachFromMouse
  (bind _returnvalue (Game|GetPlayerController 0))
  (bind _hitresult (Game|Player|GetHitResultUnderCursorbyChannel _returnvalue "TraceTypeQuery1" true))
  (bind (_bblockinghit _binitialoverlap _time _distance _location _impactpoint _normal _impactnormal) (Collision|BreakHitResult _hitresult))
  (bind _returnvalue_2 (Math|Rotator|MakeRotfromZ _impactnormal))
  ;[1 1 1] Pause the timer and stop the sponge following the mouse
  (Actor|Tick|SetActorTickEnabled false)
  (Class|KismetSystemLibrary|PauseTimer 0 "SetScrubValue")
  (Utilities|FlowControl|Gate true) ; enters at Close
)

(event EventTick
  (params (DeltaSeconds :type Float%20%28single-precision%29))
  (bind _returnvalue (Game|GetPlayerController 0))
  (bind _hitresult (Game|Player|GetHitResultUnderCursorbyChannel _returnvalue "TraceTypeQuery1" true))
  (bind (_bblockinghit _binitialoverlap _time _distance _location _impactpoint _normal _impactnormal) (Collision|BreakHitResult _hitresult))
  (bind _returnvalue_2 (Math|Rotator|MakeRotfromZ _impactnormal))
  (Utilities|FlowControl|Gate true
    (:Exit
      ;[1 1 1] Check what the mouse is hovered over and set the sponge to be on top of it.
      (Transformation|SetActorLocation _impactpoint false false)
      (Transformation|SetActorRotation (Math|Rotator|MakeRotator (.roll _returnvalue_2) 0.0 (.yaw _returnvalue_2))))))

(fn ConstructionScript)

(fn SetScrubValue
  (bind _dishtocleanref (Variables|Default|GetDishToCleanRef))
  ;[1 1 1] Check where the sponge was and where it is now and get the distance inbetween. Use that to reduce the amount of dirt on the dish
  (Variables|Default|SetScrub%20value (Math|Vector|Distance(Vector) (Variables|Default|GetLastLoc) (.ImpactPoint (Collision|BreakHitResult (.HitResult (Game|Player|GetHitResultUnderCursorbyChannel (Game|GetPlayerController 0) "TraceTypeQuery1" true))))))
  (Variables|Default|SetLastLoc (Transformation|GetActorLocation))
  (Utilities|IsValid _dishtocleanref
    (:Is%20Valid
      (Default|CleanTick _dishtocleanref))))